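; BP_Mortar is a mortar unit with a barrel, turret, aiming component and health bar widget.
; On BeginPlay it initializes MortarAiming with its TankBarrel and TankTurret.
; It then casts the HealthBar component's widget to UI_HealthBar and sets itself as that widget's OwningTank.
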(event EventBeginPlay
  (Class|TankAimingComponent|Initialize (Variables|Default|GetMortarAiming) (Variables|Default|GetTankBarrel) (Variables|Default|GetTankTurret))
  (CallFunction|InitializeHealthBarWidget))

(fn ConstructionScript)

(fn InitializeHealthBarWidget
  (bind _asui_health_bar (Utilities|Casting|CastToUI_HealthBar (UserInterface|GetUserWidgetObject (Variables|Default|GetHealthBar))))
  (Variables|/Game/UI/UI_HealthBar.UI_HealthBar_C|SetOwningTank _asui_health_bar self))